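; BP_ReactiveAudio is an actor that makes a sphere's material react to the audio it plays.
; On BeginPlay it gives the sphere a dynamic instance of M_AudioReactive and watches the MetaSound "Intensity" output on its Audio component through the MetaSound Output Subsystem.
; Each change in that output feeds the float into the material's "Audio Intensity" parameter, driving the visual from the sound without per-frame Tick polling.
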(event Custom|Update%20Material
  (params (OutputName :type Name) (Output :type Meta%20Sound%20Output%20Structure%20%28by%20ref%29))
  (bind _returnvalue (Class|MetasoundOutputBlueprintAccess|GetFloat Output))
  (Rendering|Material|SetScalarParameterValue (Variables|Default|GetAudioMaterial) "Audio Intensity" _returnvalue :!class /Script/Engine.MaterialInstanceDynamic))

(event EventBeginPlay
  (bind _returnvalue (Rendering|Material|CreateDynamicMaterialInstance (Variables|Default|GetSphere) 0 "/Game/BackgroundStuff/SmoothOperator-Sade/M_AudioReactive.M_AudioReactive" "None" :!class /Script/Engine.PrimitiveComponent))
  (bind _output_get (Variables|Default|SetAudioMaterial _returnvalue))
  (Rendering|Material|SetMaterial (Variables|Default|GetSphere) 0 _output_get)
  (MetaSoundOutput|WatchOutput (WorldSubsystems|GetMetaSoundOutputSubsystem) (Variables|Default|GetAudio) "Intensity" (delegate Custom|Update%20Material) "None" "None" :!class /Script/MetasoundEngine.MetaSoundOutputSubsystem))

(fn ConstructionScript)