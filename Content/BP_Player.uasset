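; Player Blueprint that sets up the menu UI for whichever level is loaded in what appears to be a song-based game.
; On BeginPlay it checks the current level name and creates the matching main menu, song select, settings, delay adjustment or results widget.
; Each widget gets UI-only input focused on a default button with the mouse cursor hidden.
; Pressing P opens the song select level.
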(event EventBeginPlay
  (bind _returnvalue (Game|GetPlayerController 0))
  (bind _returnvalue_2 (Game|GetPlayerController 0))
  (bind _returnvalue_3 (Game|GetPlayerController 0))
  (bind _returnvalue_4 (Game|GetPlayerController 0))
  (bind _returnvalue_5 (Game|GetPlayerController 0))
  ;[0.15 0.15 0.15 0.5] Add HUD Depending On Level
  (bind _returnvalue_6 (Game|GetCurrentLevelName true))
  (if (Utilities|Enum|Equal(Enum) _returnvalue_6 "MainMenuLevel")
    (bind _returnvalue_7 (UserInterface|CreateWidget "/Game/UI/WBP_MainMenu.WBP_MainMenu_C"))
    (bind _output_get (Variables|Default|SetMainMenuUI _returnvalue_7))
    (UserInterface|Viewport|AddtoViewport _output_get 0)
    (Variables|/Script/Engine.PlayerController|SetbShowMouseCursor _returnvalue_5 false)
    (Input|SetInputModeUIOnly _returnvalue_5 (Variables|/Game/UI/WBP_MainMenu.WBP_MainMenu_C|GetPlayButton (Variables|Default|GetMainMenuUI)) "DoNotLock" false)
    (elif (Utilities|Enum|Equal(Enum) _returnvalue_6 "SongSelectScreen")
      (bind _returnvalue_8 (UserInterface|CreateWidget "/Game/UI/WBP_SongSelector.WBP_SongSelector_C"))
      (bind _output_get_2 (Variables|Default|SetSongSelectUI _returnvalue_8))
      (UserInterface|Viewport|AddtoViewport _output_get_2 0)
      (Variables|/Script/Engine.PlayerController|SetbShowMouseCursor _returnvalue_2 false)
      (Input|SetInputModeUIOnly _returnvalue_2 (Variables|/Game/UI/WBP_SongSelector.WBP_SongSelector_C|GetBackBT (Variables|Default|GetSongSelectUI)) "DoNotLock" false)
      (elif (Utilities|Enum|Equal(Enum) _returnvalue_6 "OptionsLevel")
        (bind _returnvalue_9 (UserInterface|CreateWidget "/Game/UI/WBP_Settings.WBP_Settings_C"))
        (bind _output_get_3 (Variables|Default|SetSettingsUI _returnvalue_9))
        (UserInterface|Viewport|AddtoViewport _output_get_3 0)
        (Variables|/Script/Engine.PlayerController|SetbShowMouseCursor _returnvalue_3 false)
        (Input|SetInputModeUIOnly _returnvalue_3 (Variables|/Game/UI/WBP_Settings.WBP_Settings_C|GetBackButton (Variables|Default|GetSettingsUI)) "DoNotLock" false)
        (elif (Utilities|Enum|Equal(Enum) _returnvalue_6 "DelayAdjustmentLevel")
          (bind _returnvalue_10 (UserInterface|CreateWidget "/Game/UI/WBP_DelayAdjustment.WBP_DelayAdjustment_C"))
          (bind _output_get_4 (Variables|Default|SetDelayAdjustmentUI _returnvalue_10))
          (UserInterface|Viewport|AddtoViewport _output_get_4 0)
          (Variables|/Script/Engine.PlayerController|SetbShowMouseCursor _returnvalue_4 false)
          (Input|SetInputModeUIOnly _returnvalue_4 (Variables|/Game/UI/WBP_DelayAdjustment.WBP_DelayAdjustment_C|GetConfirmButton (Variables|Default|GetDelayAdjustmentUI)) "DoNotLock" false)
          (elif (Utilities|Enum|Equal(Enum) _returnvalue_6 "ResultsScreenLevel")
            (bind _returnvalue_11 (UserInterface|CreateWidget "/Game/UI/WBP_ResultsScreen.WBP_ResultsScreen_C"))
            (bind _output_get_5 (Variables|Default|SetResultsScreen _returnvalue_11))
            (UserInterface|Viewport|AddtoViewport _output_get_5 0)
            (Variables|/Script/Engine.PlayerController|SetbShowMouseCursor _returnvalue false)
            (Input|SetInputModeUIOnly _returnvalue (Variables|/Game/UI/WBP_ResultsScreen.WBP_ResultsScreen_C|GetRetryButton (Variables|Default|GetResultsScreen)) "DoNotLock" false)))))))

(event Collision|EventActorBeginOverlap
  (params (OtherActor :type Actor%20Object%20Reference)))

(event EventTick
  (params (DeltaSeconds :type Float%20%28single-precision%29)))

(event Input|KeyboardEvents|P
  (params (Key :type Key%20Structure :default "None"))
  (:Pressed
    (Game|OpenLevel(byName) "SongSelectScreen")))

(fn ConstructionScript)