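; BP_Note1 is a rhythm-game note that travels along the first lane spline of the level's BP_Spline actor.
; On BeginPlay it caches that spline actor.
; MoveNotes picks a random direction from four, applies the matching arrow material to its sphere and starts a timeline scaled by TimeToComplete.
; Each timeline update places the note by distance along Lane01, using the spline's local-space location and rotation.
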(event Custom|MoveNotes
  (bind _rhythmspline (Variables|Default|GetRhythmSpline))
  (bind _sphere (Variables|Default|GetSphere))
  (bind _lane_01 (Variables|/Game/BP_Spline.BP_Spline_C|GetLane_01 _rhythmspline))
  ;[0.15 0.15 0.15 0.5] Assign Arrow Direction and Assign Correct Material
  (bind _output_get (Variables|Default|SetDirection%20Value (Math|Random|RandomIntegerinRange 1 4)))
  (if (== _output_get 1)
    (Rendering|Material|SetMaterial _sphere 0 "/Game/ArrowMats/Arrow1_Mat.Arrow1_Mat")
    (elif (== _output_get 2)
      (Rendering|Material|SetMaterial _sphere 0 "/Game/ArrowMats/Arrow2_Mat.Arrow2_Mat")
      (elif (== _output_get 3)
        (Rendering|Material|SetMaterial _sphere 0 "/Game/ArrowMats/Arrow3_Mat.Arrow3_Mat")
        (else
          (Rendering|Material|SetMaterial _sphere 0 "/Game/ArrowMats/Arrow4_Mat.Arrow4_Mat")))))
  (Components|Timeline|SetPlayRate (Variables|Default|GetTimeline) (/ 1.0 (Variables|Default|GetTimeToComplete)))
  (bind _newtrack_0 (Timeline|Timeline PlayFromStart)
    (:Update
      (Transformation|SetActorTransform (Math|Transform|MakeTransform (Spline|GetLocationatDistanceAlongSpline _lane_01 (Math|Float|Lerp 0.0 (Spline|GetSplineLength (Variables|/Game/BP_Spline.BP_Spline_C|GetLane_01 (Variables|Default|GetRhythmSpline))) _newtrack_0) "Local") (Spline|GetRotationatDistanceAlongSpline _lane_01 (Math|Float|Lerp 0.0 (Spline|GetSplineLength (Variables|/Game/BP_Spline.BP_Spline_C|GetLane_01 (Variables|Default|GetRhythmSpline))) _newtrack_0) "Local") (Variables|/Script/Engine.SceneComponent|GetRelativeScale3D (Variables|Default|GetSphere)))))))

(event EventBeginPlay
  (bind _returnvalue (Actor|GetActorOfClass "/Game/BP_Spline.BP_Spline_C"))
  (Variables|Default|SetRhythmSpline _returnvalue))

(fn ConstructionScript)